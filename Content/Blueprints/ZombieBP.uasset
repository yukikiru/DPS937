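; Zombie enemy Blueprint that chases the player on sight and attacks in melee.
; PawnSensing casts the seen pawn to PlayerBP, clears idle and starts AIMoveTo unless mid-attack.
; A self-repeating Delay loop keeps yawing the zombie toward player pawn 0.
; Reaching the target subtracts Health directly from the player, with an IsAttack flag held briefly as a cooldown.
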(event `self.ReceiveTick`
  (params (DeltaSeconds :type "Float (single-precision)"))
  ;[1 1 1] On Sight, follow and look at player
)

(event `self.PawnSensing.OnSeePawn`
  (params (Pawn :type "Pawn Object Reference"))
  (bind _theplayer (`self.ThePlayer`))
  ;[1 1 1] On Sight, follow and look at player
  (bind _asplayer_bp (cast `/Game/Blueprints/PlayerBP` Pawn))
  (bind _output_get (set `self.ThePlayer` _asplayer_bp))
  (set `self.isIdle` false)
  (if (== (`self.isAttack`) false)
    (`|AIMoveTo` self (0.0 0.0 0.0) _output_get 30.0
      (:`then`
        (`self.K2_SetActorRotation` (`KismetMathLibrary.MakeRotator` 0.0 0.0 (.yaw (`KismetMathLibrary.FindLookAtRotation` (`SceneComponent.K2_GetComponentLocation` (`self.Mesh`)) (`self.K2_GetActorLocation` (`GameplayStatics.GetPlayerPawn` 0))))) :!label _label)
        (`KismetSystemLibrary.Delay` (stale `self.ReceiveTick` DeltaSeconds))
        (goto _label))
      (:`OnSuccess`
        ;[1 1 1] Attack Player
        (set `self.isAttack` true)
        (set `/Game/Blueprints/PlayerBP.Health` (- (`/Game/Blueprints/PlayerBP.Health` _theplayer) 25.0) _theplayer)
        (`KismetSystemLibrary.Delay` 0.5)
        (set `self.isAttack` false)))))

(fn `UserConstructionScript`)
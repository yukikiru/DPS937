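; Interactive gate actor that swings open and closed when the player presses E inside its trigger volume.
; Trigger overlap enables input and shows a Press E widget; leaving disables input and removes all widgets.
; E flips IsOpen and plays or reverses the DoorRotation timeline, whose yaw is combined with the rotation saved at BeginPlay.
; Overlap events do not filter which actor enters or leaves.
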(event `self.ReceiveBeginPlay`
  (set `self.doorInit` (`self.K2_GetActorRotation`))
  (bind _returnvalue (`|CreateWidget` "/Game/Blueprints/Widgets/Press_E.Press_E_C" (`GameplayStatics.GetPlayerController` 0))))

(event `self.Trigger.OnComponentBeginOverlap`
  (params (OverlappedComponent :type "PrimitiveComponent Object Reference") (OtherActor :type "Actor Object Reference") (OtherComp :type "PrimitiveComponent Object Reference") (OtherBodyIndex :type Integer) (bFromSweep :type Boolean) (SweepResult :type "HitResult Structure (by ref)"))
  (`self.EnableInput` (`GameplayStatics.GetPlayerController` 0))
  (`UserWidget.AddToViewport` (stale `self.ReceiveBeginPlay` _returnvalue) 0))

(event `Key|E`
  (params (Key :type "Key Structure"))
  (:`Pressed`
    (if (`self.isOpen`)
      (set `self.isOpen` false)
      (bind (_direction _doorrotation) (`Timeline|DoorRotation` :!label _label)
        (:`Update`
          (`self.K2_SetActorRelativeRotation` (`KismetMathLibrary.ComposeRotators` (`KismetMathLibrary.MakeRotator` 0.0 0.0 _doorrotation) (`self.doorInit`)))))
      (else
        (set `self.isOpen` true)
        (goto _label :!via `Reverse`)))))

(event `self.Trigger.OnComponentEndOverlap`
  (params (OverlappedComponent :type "PrimitiveComponent Object Reference") (OtherActor :type "Actor Object Reference") (OtherComp :type "PrimitiveComponent Object Reference") (OtherBodyIndex :type Integer))
  (`self.DisableInput` (`GameplayStatics.GetPlayerController` 0))
  (`WidgetLayoutLibrary.RemoveAllWidgets`))

(fn `UserConstructionScript`)
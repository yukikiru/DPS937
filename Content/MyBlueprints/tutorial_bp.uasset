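; A tutorial Blueprint that makes its point light flicker between very bright and nearly off.
; BeginPlay prints a colored debug string and sets the Intensity boolean to true.
; Each Tick runs a FlipFlop that alternates the light between high and minimal intensity while that boolean holds, so the flicker rate follows the frame rate.
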(event `self.ReceiveBeginPlay`
  (`KismetSystemLibrary.PrintString` "Hello" true true (struct :`R` 1.0 :`G` 0.04246 :`B` 0.172208 :`A` 1.0))
  (set `self.intensity` true))

(event `self.ReceiveTick`
  (params (DeltaSeconds :type "Float (single-precision)"))
  (`/Engine/EditorBlueprintResources/StandardMacros.FlipFlop`
    (:`A`
      (if (`self.intensity`)
        (`LightComponent.SetIntensity` (`self.PointLight`) 50000.0)))
    (:`B`
      (if (`self.intensity`)
        (`LightComponent.SetIntensity` (`self.PointLight`) 1.0)))))

(fn `UserConstructionScript`)